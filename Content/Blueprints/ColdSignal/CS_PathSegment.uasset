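; CS_PathSegment is a path segment actor with a guide line that boosts a FlyingPawn's thrust and glows brighter while the pawn overlaps its trigger.
; The construction script rebuilds a straight row of evenly spaced instanced static meshes along X.
; Trigger begin and end overlaps switch the pawn's thrust multiplier and an emissive target between high and low values.
; Tick lerps the guide line's dynamic material EmissivePower toward that target for a smooth fade.
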(event `self.ReceiveBeginPlay`
  (bind _returnvalue (`PrimitiveComponent.CreateDynamicMaterialInstance` (`self.GuideLine1`) 0 "/Game/Blueprints/ColdSignal/MI_GuideLine.MI_GuideLine"))
  (set `self.GL1DynamicMaterial` _returnvalue))

(event `self.ReceiveTick`
  (params (DeltaSeconds :type "Float (single-precision)"))
  (bind _gl1dynamicmaterial (`self.GL1DynamicMaterial`))
  (`|ExecutionSequence`
    (:`then_0`
      (bind _returnvalue (`MaterialInstanceDynamic.K2_GetScalarParameterValue` _gl1dynamicmaterial "EmissivePower"))
      (`MaterialInstanceDynamic.SetScalarParameterValue` _gl1dynamicmaterial "EmissivePower" (`KismetMathLibrary.Lerp` _returnvalue (`self.GL1EmissiveTarget`) (* DeltaSeconds (`self.EmitLerpRate`)))))))

(event `self.GuideLine1Trigger.OnComponentBeginOverlap`
  (params (OverlappedComponent :type "PrimitiveComponent Object Reference") (OtherActor :type "Actor Object Reference") (OtherComp :type "PrimitiveComponent Object Reference") (OtherBodyIndex :type Integer) (bFromSweep :type Boolean) (SweepResult :type "HitResult Structure (by ref)"))
  (bind _asflying_pawn (cast `/Game/Blueprints/FlyingPawn` OtherActor))
  (set `/Game/Blueprints/FlyingPawn.ThrustMultiplier` 10000.0 _asflying_pawn)
  (set `self.GL1EmissiveTarget` 50.0))

(event `self.GuideLine1Trigger.OnComponentEndOverlap`
  (params (OverlappedComponent :type "PrimitiveComponent Object Reference") (OtherActor :type "Actor Object Reference") (OtherComp :type "PrimitiveComponent Object Reference") (OtherBodyIndex :type Integer))
  (bind _asflying_pawn (cast `/Game/Blueprints/FlyingPawn` OtherActor))
  (set `/Game/Blueprints/FlyingPawn.ThrustMultiplier` 1000.0 _asflying_pawn)
  (set `self.GL1EmissiveTarget` 10.0))

(fn `UserConstructionScript`
  (`InstancedStaticMeshComponent.ClearInstances` (`self.InstancedStaticMesh`))
  (for _index (range 40)
    (`InstancedStaticMeshComponent.AddInstance` (`self.InstancedStaticMesh`) (`KismetMathLibrary.MakeTransform` (`KismetMathLibrary.MakeVector` (* _index 82700.0)) (struct)))))