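; TwistingLumpyTorus is an actor Blueprint that rises vertically once its StartMoving event fires.
; StartMoving records the current height as StartZ and sets ShouldMove.
; Tick then raises the actor along world Z at MoveIncrement scaled by delta time until it reaches StartZ plus TotalMoveDistanceZ, leaving X and Y unchanged.
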(event `self.ReceiveTick`
  (params (DeltaSeconds :type "Float (single-precision)"))
  (bind (_returnvalue_x _returnvalue_y _returnvalue_z) (`KismetMathLibrary.BreakVector` (`self.K2_GetActorLocation`)))
  (bind (_returnvalue_x_2 _returnvalue_y_2 _returnvalue_z_2) (`KismetMathLibrary.BreakVector` (`self.K2_GetActorLocation`)))
  (if (`self.ShouldMove`)
    (if (< _returnvalue_z_2 (+ (`self.StartZ`) (`self.TotalMoveDistanceZ`)))
      (`self.K2_SetActorLocation` (`KismetMathLibrary.MakeVector` _returnvalue_x _returnvalue_y (+ _returnvalue_z (* (`self.MoveIncrement`) (`GameplayStatics.GetWorldDeltaSeconds`))))))))

(event `StartMoving`
  (bind (_returnvalue_x _returnvalue_y _returnvalue_z) (`KismetMathLibrary.BreakVector` (`self.K2_GetActorLocation`)))
  (set `self.StartZ` _returnvalue_z)
  (set `self.ShouldMove` true))

(fn `UserConstructionScript`)