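; FloatingSphere is an actor whose sphere mesh drifts along its local Z axis once StartMoving is called.
; The construction script randomizes each scale axis independently, allowing uneven shapes, and picks a random speed within set bounds.
; Tick applies a swept local offset that multiplies speed by delta time twice, so movement depends on frame rate.
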(event `self.ReceiveTick`
  (params (DeltaSeconds :type "Float (single-precision)"))
  (if (`self.ShouldMove`)
    (`self.K2_AddActorLocalOffset` (`KismetMathLibrary.MakeVector` 0.0 0.0 (* (* DeltaSeconds (`self.Speed`)) (`GameplayStatics.GetWorldDeltaSeconds`))) true)))

(event `StartMoving`
  (set `self.ShouldMove` true))

(fn `UserConstructionScript`
  (bind _returnvalue (`KismetMathLibrary.RandomFloatInRange` (`self.MinSize`) (`self.MaxSize`)))
  (`SceneComponent.SetWorldScale3D` (`self.SphereMesh`) (`KismetMathLibrary.MakeVector` _returnvalue _returnvalue _returnvalue))
  (set `self.Speed` (`KismetMathLibrary.RandomFloatInRange` (`self.MinSpeed`) (`self.MaxSpeed`))))